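; BP_TriggerPlatform_Are is a one-shot trigger platform that swaps the ThomasTestingPhysicsShit actor that touches it for a playable BP_Pistol.
; On overlap it destroys that actor, spawns a BP_Pistol above its Hitbox with the old actor's roll and yaw but zero pitch, and has player controller 0 possess it.
; A TriggeredOnce flag blocks repeat swaps, and later overlaps only print a debug message.
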(event EventBeginPlay)

(event Collision|EventActorBeginOverlap
  (params (OtherActor :type Actor%20Object%20Reference))
  (if (Variables|Default|GetbTriggeredOnce)
    (Development|PrintString "Allready Triggered TriggerPlatform")
    (else
      (bind _asthomas_testing_physics_shit (Utilities|Casting|CastToThomasTestingPhysicsShit OtherActor))
      (Variables|Default|Setforwardrotation (Transformation|GetActorRotation _asthomas_testing_physics_shit))
      (Actor|DestroyActor _asthomas_testing_physics_shit)
      (bind _returnvalue (Game|SpawnActorfromClass "/Game/PlayerCharacter/BP_Pistol.BP_Pistol_C" (Math|Conversions|ToTransform(Vector) (+ (Transformation|GetWorldLocation (Variables|Default|GetHitbox)) "11.000000, 0,100.000000")) "AdjustIfPossibleButAlwaysSpawn" (Game|Player|GetPlayerPawn 0) 0.0 0))
      (Transformation|SetActorRotation _returnvalue (Math|Rotator|MakeRotator (.Roll (Math|Rotator|BreakRotator (Variables|Default|Getforwardrotation))) 0.0 (.Yaw (Math|Rotator|BreakRotator (Variables|Default|Getforwardrotation)))))
      (Pawn|Possess (Game|GetPlayerController 0) _returnvalue)
      (Variables|Default|SetbTriggeredOnce true))))

(event EventTick
  (params (DeltaSeconds :type Float%20%28single-precision%29)))

(fn ConstructionScript)