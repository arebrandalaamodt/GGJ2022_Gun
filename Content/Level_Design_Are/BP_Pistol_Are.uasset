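; Player-controlled pistol pawn that moves, aims and fires a charged shot, then hands control to the projectile.
; Movement follows control yaw; holding Aim collapses the spring arm, raises the actor and enables pitch look, while release restores the chase camera.
; Holding Shoot builds capped power on Tick to set projectile velocity.
; Releasing it spawns and possesses a ThomasTestingPhysicsShit, plays the fire animation and destroys the pawn after a short delay.
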(event EventBeginPlay
  (Transformation|SetRelativeLocation (Variables|Default|GetSpringArm) "0, 0, 0" false false))

(event Collision|EventActorBeginOverlap
  (params (OtherActor :type Actor%20Object%20Reference)))

(event EventTick
  (params (DeltaSeconds :type Float%20%28single-precision%29))
  (if (<= (Variables|Character|GetPowerOfBullet) 1e+02)
    (if (Variables|Default|GetIsChargingPower)
      (bind _output_get (Variables|Character|SetPowerOfBullet (+ (Variables|Character|GetPowerOfBullet) (* DeltaSeconds 75.0)))))))

(event Input|ActionEvents|InputActionAim
  (params (Key :type Key%20Structure :default "None"))
  (bind _springarm (Variables|Default|GetSpringArm))
  (bind _springarm_2 (Variables|Default|GetSpringArm))
  (:Pressed
    (Variables|Default|SetIsAiming true)
    (Variables|/Script/Engine.SpringArmComponent|SetTargetArmLength _springarm_2 0.0)
    (Variables|/Script/Engine.SpringArmComponent|SetTargetOffset _springarm_2 "0, 0, 0")
    (Transformation|AddActorLocalOffset "0, 0,50.000000" false false))
  (:Released
    (Variables|Default|SetIsAiming false)
    (Pawn|SetControlRotation (Game|GetPlayerController 0) (Math|Rotator|MakeRotator 0.0 0.0 (.Yaw (Math|Rotator|BreakRotator (Pawn|GetControlRotation :!class /Script/Engine.Pawn)))))
    (Variables|/Script/Engine.SpringArmComponent|SetTargetArmLength _springarm 3e+02)
    (Variables|/Script/Engine.SpringArmComponent|SetTargetOffset _springarm "0, 0,100.000000")))

(event Input|ActionEvents|InputActionShoot
  (params (Key :type Key%20Structure :default "None"))
  (:Pressed
    (if (not (Variables|Default|GetIsChargingPower))
      (Variables|Default|SetIsChargingPower true)))
  (:Released
    (if (Variables|Default|GetIsAiming)
      _
      (else
        _))
    (Variables|Default|SetIsChargingPower false)
    (bind _returnvalue (Game|SpawnActorfromClass "/Game/BulletCharacter/ThomasTestingPhysicsShit.ThomasTestingPhysicsShit_C" (Math|Transform|MakeTransform (Transformation|GetWorldLocation (Variables|Default|GetBulletSpawnPoint)) (Transformation|GetActorRotation) "1,1,1") "Undefined" 0 (+ (Variables|Default|GetMinForce) (* (Variables|Character|GetPowerOfBullet) 15.0)) self))
    (Variables|Character|SetPowerOfBullet 0.0)
    (Components|Animation|PlayAnimation (Variables|Character|GetMesh) "/Game/PlayerCharacter/GunMan_Animated_Anim_lul_Fire.GunMan_Animated_Anim_lul_Fire" false)
    (Pawn|Possess (Game|GetPlayerController 0) _returnvalue)
    (Utilities|FlowControl|Delay 0.6)
    (Actor|DestroyActor)
    (Variables|Default|SetIsChargingPower false)))

(event Input|AxisEvents|InputAxisForward
  (params (AxisValue :type Float%20%28single-precision%29))
  (Pawn|Input|AddMovementInput (Math|Vector|GetForwardVector (Math|Rotator|MakeRotator 0.0 0.0 (.Yaw (Math|Rotator|BreakRotator (Pawn|GetControlRotation :!class /Script/Engine.Pawn))))) AxisValue false))

(event Input|AxisEvents|InputAxisSideways
  (params (AxisValue :type Float%20%28single-precision%29))
  (Pawn|Input|AddMovementInput (Math|Vector|GetRightVector (Math|Rotator|MakeRotator 0.0 0.0 (.Yaw (Math|Rotator|BreakRotator (Pawn|GetControlRotation :!class /Script/Engine.Pawn))))) AxisValue false))

(event Input|AxisEvents|InputAxisTurn
  (params (AxisValue :type Float%20%28single-precision%29))
  (Pawn|Input|AddControllerYawInput AxisValue))

(event Input|AxisEvents|InputAxisLookUp
  (params (AxisValue :type Float%20%28single-precision%29))
  (if (Variables|Default|GetIsAiming)
    (Pawn|Input|AddControllerPitchInput AxisValue)))

(fn ConstructionScript)