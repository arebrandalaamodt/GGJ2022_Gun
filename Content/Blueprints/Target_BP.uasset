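; Target_BP is a target that swaps the overlapping ThomasTestingPhysicsShit actor for a player-controlled BP_Pistol.
; On overlap with that class it plays an explosion sound at the target, spawns the pistol at the actor's transform and destroys the actor.
; The pistol keeps the old roll and yaw with pitch zeroed, then player controller 0 possesses it.
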(event EventBeginPlay)

(event Collision|EventActorBeginOverlap
  (params (OtherActor :type Actor%20Object%20Reference))
  (bind _asthomas_testing_physics_shit (Utilities|Casting|CastToThomasTestingPhysicsShit OtherActor))
  (Variables|Default|Setforwardrotation (Transformation|GetActorRotation _asthomas_testing_physics_shit))
  (Audio|PlaySoundatLocation "/Game/StarterContent/Audio/Explosion01.Explosion01" (Transformation|GetActorLocation) "0, 0, 0" 1.0 1.0 0.0 0 0 0)
  (bind _returnvalue (Game|SpawnActorfromClass "/Game/PlayerCharacter/BP_Pistol.BP_Pistol_C" (Transformation|GetActorTransform _asthomas_testing_physics_shit) "AdjustIfPossibleButAlwaysSpawn" (Game|Player|GetPlayerPawn 0) 0.0 0))
  (Actor|DestroyActor _asthomas_testing_physics_shit)
  (Transformation|SetActorRotation _returnvalue (Math|Rotator|MakeRotator (.Roll (Math|Rotator|BreakRotator (Variables|Default|Getforwardrotation))) 0.0 (.Yaw (Math|Rotator|BreakRotator (Variables|Default|Getforwardrotation)))))
  (Pawn|Possess (Game|GetPlayerController 0) _returnvalue))

(fn ConstructionScript)