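; BP_DeadlyWater is a rising hazard that sends the player back to a spawn point and resets its own height.
; It stores its start location and plays a fire sound on BeginPlay, then climbs a fixed step every Tick, independent of delta time.
; Any overlap with its Box resets the root to the start and teleports the player's BP_Pistol pawn to Spawnpoint, without checking what overlapped.
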(event OnComponentBeginOverlap(Box)
  (params (OverlappedComponent :type Primitive%20Component%20Object%20Reference) (OtherActor :type Actor%20Object%20Reference) (OtherComp :type Primitive%20Component%20Object%20Reference) (OtherBodyIndex :type Integer) (bFromSweep :type Boolean) (SweepResult :type Hit%20Result%20Structure%20%28by%20ref%29))
  (Transformation|SetWorldLocation (Variables|Default|GetDefaultSceneRoot) (Variables|Default|GetStartLocation) false false)
  (bind _asbp_pistol (Utilities|Casting|CastToBP_Pistol (Game|Player|GetPlayerPawn 0)))
  (Transformation|SetActorLocation _asbp_pistol (Transformation|GetWorldLocation (Variables|Default|GetSpawnpoint)) false false))

(event EventBeginPlay
  (bind _returnvalue (Transformation|GetActorLocation))
  (Audio|PlaySoundatLocation "/Game/StarterContent/Audio/Fire01.Fire01" _returnvalue "0, 0, 0" 1.0 1.0 0.0 0 0 0)
  (Variables|Default|SetStartLocation _returnvalue))

(event Collision|EventActorBeginOverlap
  (params (OtherActor :type Actor%20Object%20Reference)))

(event EventTick
  (params (DeltaSeconds :type Float%20%28single-precision%29))
  (Transformation|AddLocalOffset (Variables|Default|GetDefaultSceneRoot) "0, 0,1.000000" false false))

(fn ConstructionScript)